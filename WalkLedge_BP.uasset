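; Placeable wall-ledge segment that the ACF player shuffles along, chainable to neighbours through front/back references keyed by corner type.
; End trigger overlaps snap the player into a ledge-walk moveset, play corner or exit montages, and hand off or clear the player's ledge reference via BreakLinkToLedge.
; Montage-end callback re-enables input after entry.
; Construction script optionally stretches the segment by DistanceVector; the PositionChecker alignment validator is never called.
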(event OnComponentBeginOverlap(Entrance)
  (params (OverlappedComponent :type Primitive%20Component%20Object%20Reference) (OtherActor :type Actor%20Object%20Reference) (OtherComp :type Primitive%20Component%20Object%20Reference) (OtherBodyIndex :type Integer) (bFromSweep :type Boolean) (SweepResult :type Hit%20Result%20Structure%20%28by%20ref%29))
  (bind _start_end_point (Variables|Default|GetStart/End%20Point))
  (bind _ledgereference_back_ (Variables|LedgeSets|GetLedgeReference%28Back%29))
  (bind _reversedirection (Variables|LedgeSets|GetReverseDirection))
  (bind _returnvalue (Transformation|GetWorldLocation _start_end_point))
  (bind _returnvalue_2 (Utilities|Map|Length _ledgereference_back_))
  (bind _returnvalue_3 (== _returnvalue_2 0))
  ;[1 1 1] Entrance Trigger Begin OverlaComment
  (bind _asacf_my_current (Utilities|Casting|CastToACF_My_Current OtherActor))
  (Variables|Default|GetAs%20ACF%20My%20Current
    (:then
      _)
    (:else
      (Variables|Default|SetAs%20ACF%20My%20Current _asacf_my_current)))
  (if (AI|Components|NavMovement|IsMovingonGround (Variables|/Script/Engine.Character|GetCharacterMovement (Variables|Default|GetAs%20ACF%20My%20Current)))
    (if (or (Animation|Montage|MontageIsPlaying (Class|ACFCharacter|GetACFAnimInstance (Variables|Default|GetAs%20ACF%20My%20Current)) "/Game/RetargetAnimations/TraversalAnimations/Traversal_LedgeWalk/RM/Montages/RightLedgeWalk.RightLedgeWalk") (Animation|Montage|MontageIsPlaying (Class|ACFCharacter|GetACFAnimInstance (Variables|Default|GetAs%20ACF%20My%20Current)) "/Game/RetargetAnimations/TraversalAnimations/Traversal_LedgeWalk/RM/Montages/Left/LeftLedgeWalk.LeftLedgeWalk"))
      (if (Variables|Default|GetOnLedge) :!label _label
        (if (Variables|Default|GetStart/End%20Ledge?)
          ;;[0 1 0.2437] When we are in the starting ledge only
          (if (== (Utilities|Map|Length (Variables|LedgeSets|GetLedgeReference%28Front%29)) 0)
            (if _returnvalue_3
              ;;;[1 0.4626 0] This section only happen if there are no back or forward ledge references set
              (|SwitchGameplayTag (Class|ACFCharacter|GetCurrentMoveset (Variables|Default|GetAs%20ACF%20My%20Current))
                (:Movesets.LedgeWalk
                  (Animation|PlayAnimMontage (Variables|Default|GetAs%20ACF%20My%20Current) "/Game/RetargetAnimations/TraversalAnimations/Traversal_LedgeWalk/RM/Montages/Left/LedgeLeft_End.LedgeLeft_End" 1.0 "None"))
                (:Movesets.LedgeWalkRight
                  (Animation|PlayAnimMontage (Variables|Default|GetAs%20ACF%20My%20Current) "/Game/RetargetAnimations/TraversalAnimations/Traversal_LedgeWalk/RM/Montages/LedgeRight_End.LedgeRight_End" 1.0 "None")))
              (CallFunction|BreakLinktoLedge false false)
              (elif (.ReturnValue (Utilities|Map|Find (Variables|LedgeSets|GetLedgeReference%28Back%29) (Variables|LedgeSets|GetReverseDirection)))
                (switch Utilities|FlowControl|Switch|SwitchonWalkLedge_Directions_Enum (Variables|LedgeSets|GetReverseDirection)
                  (:NewEnumerator0
                    (Animation|PlayAnimMontage (Variables|Default|GetAs%20ACF%20My%20Current) "/Game/RetargetAnimations/TraversalAnimations/Traversal_LedgeWalk/RM/Montages/LedgeRight_Inner_Corner.LedgeRight_Inner_Corner" 1.0 "None"))
                  (:NewEnumerator3
                    (Animation|PlayAnimMontage (Variables|Default|GetAs%20ACF%20My%20Current) "/Game/RetargetAnimations/TraversalAnimations/Traversal_LedgeWalk/RM/Montages/LedgeRight_Outer_Corner.LedgeRight_Outer_Corner" 1.0 "None")))
                (Variables|Default|SetOnLedge false)
                (CallFunction|BreakLinktoLedge true false)))
            (elif _returnvalue_3
              ;;;[1 1 1] Means we're at the end or beginning
              (Animation|PlayAnimMontage (Variables|Default|GetAs%20ACF%20My%20Current) "/Game/RetargetAnimations/TraversalAnimations/Traversal_LedgeWalk/RM/Montages/LedgeRight_End.LedgeRight_End" 1.0 "None")
              (CallFunction|BreakLinktoLedge false false)
              (else
                (Development|PrintString "ERROR BECAUSE BOTH LEDGE REFERENCES CANNOT BE VALID ON A START LEDGE (WALKLEDGE_BP::ENTRANCE OVERLAP EVENT)" false true "(R=0.022174,G=0.003677,B=0.004391,A=1.000000)" 22.0))))
          (else
            (Utilities|IsValid (.Value (Utilities|Map|Find (Variables|LedgeSets|GetLedgeReference%28Back%29) _reversedirection))
              (:Is%20Valid
                (switch Utilities|FlowControl|Switch|SwitchonWalkLedge_Directions_Enum _reversedirection
                  (:NewEnumerator0
                    (Animation|PlayAnimMontage (Variables|Default|GetAs%20ACF%20My%20Current) "/Game/RetargetAnimations/TraversalAnimations/Traversal_LedgeWalk/RM/Montages/LedgeRight_Inner_Corner.LedgeRight_Inner_Corner" 1.0 "None"))
                  (:NewEnumerator3
                    (Animation|PlayAnimMontage (Variables|Default|GetAs%20ACF%20My%20Current) "/Game/RetargetAnimations/TraversalAnimations/Traversal_LedgeWalk/RM/Montages/LedgeRight_Outer_Corner.LedgeRight_Outer_Corner" 1.0 "None")))
                (CallFunction|BreakLinktoLedge true false)))))
        (elif (not (Variables|/Game/ACF_Assets/ACF_My_Current.ACF_My_Current_C|GetOnWalkingLedge (Variables|Default|GetAs%20ACF%20My%20Current))) ; If false then we are initializing our actor to get on its first ledge reference
          (Development|PrintString "Not on ledge. Initializing" false true "(R=0.343750,G=0.320822,B=0.335595,A=1.000000)" 7.0)
          (Components|Movement|StopMovementImmediately (Variables|/Script/Engine.Character|GetCharacterMovement (Variables|Default|GetAs%20ACF%20My%20Current)))
          (Input|DisableInput (Variables|Default|GetAs%20ACF%20My%20Current) (Game|GetPlayerController 0))
          (Transformation|SetActorLocation (Variables|Default|GetAs%20ACF%20My%20Current) (Math|Vector|MakeVector (.x _returnvalue) (.y _returnvalue) (.z (Transformation|GetActorLocation (Variables|Default|GetAs%20ACF%20My%20Current)))) false false)
          (Variables|/Script/Engine.PlayerController|SetInputYawScale (Game|GetPlayerController 0) 0.0)
          (Pawn|SetControlRotation (Game|GetPlayerController 0) (Math|Rotator|MakeRotator 0.0 0.0 (.yaw (Transformation|GetActorRotation))))
          (Utilities|FlowControl|Delay 0.8)
          (Variables|Default|SetOnLedge true)
          (Animation|PlayAnimMontage (Variables|Default|GetAs%20ACF%20My%20Current) "/Game/RetargetAnimations/TraversalAnimations/Traversal_LedgeWalk/RM/Montages/Left/LedgeLeftStart_Montage.LedgeLeftStart_Montage" 1.0 "None")
          (Class|ACFCharacter|SwitchMoveset (Variables|Default|GetAs%20ACF%20My%20Current) "(TagName=\"Movesets.LedgeWalk\")")
          (Variables|/Game/ACF_Assets/ACF_My_Current.ACF_My_Current_C|SetWalkLedge_Ref (Variables|Default|GetAs%20ACF%20My%20Current) self)))
      (elif (not (Class|AnimInstance|IsAnyMontagePlaying (Class|ACFCharacter|GetACFAnimInstance (Variables|Default|GetAs%20ACF%20My%20Current))))
        (goto _label)))))

(event OnComponentBeginOverlap(CollisionTrigger)
  (params (OverlappedComponent :type Primitive%20Component%20Object%20Reference) (OtherActor :type Actor%20Object%20Reference) (OtherComp :type Primitive%20Component%20Object%20Reference) (OtherBodyIndex :type Integer) (bFromSweep :type Boolean) (SweepResult :type Hit%20Result%20Structure%20%28by%20ref%29))
  (bind _collisiontrigger (Variables|Default|GetCollisionTrigger))
  (bind _collisiontrigger_2 (Variables|Default|GetCollisionTrigger))
  (bind _returnvalue (Transformation|GetWorldLocation _collisiontrigger_2))
  (bind _returnvalue_2 (Transformation|GetWorldRotation _collisiontrigger_2))
  (bind _returnvalue_3 (Math|Vector|GetRightVector _collisiontrigger_2))
  (bind _returnvalue_4 (Math|Vector|GetForwardVector _returnvalue_2))
  (bind _returnvalue_5 (* _returnvalue_3 4e+01))
  (bind _returnvalue_6 (* _returnvalue_4 55.0))
  (bind _returnvalue_7 (+ _returnvalue_6 _returnvalue _returnvalue_5))
  (bind (_x _y) (Math|Vector|BreakVector _returnvalue_7))
  ;[1 0 0.8418] End trigger begin overlap
  (if (Variables|Default|GetOnLedge)
    (if (or (Animation|Montage|MontageIsPlaying (Class|ACFCharacter|GetACFAnimInstance (Variables|Default|GetAs%20ACF%20My%20Current)) "/Game/RetargetAnimations/TraversalAnimations/Traversal_LedgeWalk/RM/Montages/Left/LeftLedgeWalk.LeftLedgeWalk") (Animation|Montage|MontageIsPlaying (Class|ACFCharacter|GetACFAnimInstance (Variables|Default|GetAs%20ACF%20My%20Current)) "/Game/RetargetAnimations/TraversalAnimations/Traversal_LedgeWalk/RM/Montages/RightLedgeWalk_Reversal.RightLedgeWalk_Reversal")) ; If walking montages are playing continue logic
      (if (Variables|Default|GetStart/End%20Ledge?) :!label _label
        (if (== (Utilities|Map|Length (Variables|LedgeSets|GetLedgeReference%28Front%29)) 0)
          (if (== (Utilities|Map|Length (Variables|LedgeSets|GetLedgeReference%28Back%29)) 0)
            (Variables|Default|SetOnLedge false)
            (|SwitchGameplayTag (Class|ACFCharacter|GetCurrentMoveset (Variables|Default|GetAs%20ACF%20My%20Current))
              (:Movesets.LedgeWalk
                (Animation|PlayAnimMontage (Variables|Default|GetAs%20ACF%20My%20Current) "/Game/RetargetAnimations/TraversalAnimations/Traversal_LedgeWalk/RM/Montages/Left/LedgeLeft_End.LedgeLeft_End" 1.0 "None"))
              (:Movesets.LedgeWalkRight
                (Animation|PlayAnimMontage (Variables|Default|GetAs%20ACF%20My%20Current) "/Game/RetargetAnimations/TraversalAnimations/Traversal_LedgeWalk/RM/Montages/LedgeRight_End.LedgeRight_End" 1.0 "None")))
            (CallFunction|BreakLinktoLedge false false)
            (else
              (Animation|PlayAnimMontage (Variables|Default|GetAs%20ACF%20My%20Current) "/Game/RetargetAnimations/TraversalAnimations/Traversal_LedgeWalk/RM/Montages/Left/LedgeLeft_End.LedgeLeft_End" 1.0 "None")
              (CallFunction|BreakLinktoLedge false false)))
          (else
            (Animation|PlayAnimMontage (Variables|Default|GetAs%20ACF%20My%20Current) "/Game/RetargetAnimations/TraversalAnimations/Traversal_LedgeWalk/RM/Montages/Left/LedgeLeft_Inner_Corner.LedgeLeft_Inner_Corner" 1.0 "None")
            (CallFunction|BreakLinktoLedge true true)))
        (else
          (Utilities|IsValid (.Value (Utilities|Map|Find (Variables|LedgeSets|GetLedgeReference%28Front%29) (Variables|LedgeSets|GetLedgeSelector)))
            (:Is%20Valid
              (switch Utilities|FlowControl|Switch|SwitchonWalkLedge_Directions_Enum (Variables|LedgeSets|GetLedgeSelector)
                (:NewEnumerator1
                  (Animation|PlayAnimMontage (Variables|Default|GetAs%20ACF%20My%20Current) "/Game/RetargetAnimations/TraversalAnimations/Traversal_LedgeWalk/RM/Montages/Left/LedgeLeft_Outer_Corner.LedgeLeft_Outer_Corner" 1.0 "None"))
                (:NewEnumerator2
                  (Animation|PlayAnimMontage (Variables|Default|GetAs%20ACF%20My%20Current) "/Game/RetargetAnimations/TraversalAnimations/Traversal_LedgeWalk/RM/Montages/Left/LedgeLeft_Inner_Corner.LedgeLeft_Inner_Corner" 1.0 "None")))
              (CallFunction|BreakLinktoLedge true true)))))
      (elif (not (Class|AnimInstance|IsAnyMontagePlaying (Class|ACFCharacter|GetACFAnimInstance (Variables|Default|GetAs%20ACF%20My%20Current)))) ; If any montage is playing stop, if not continue
        (goto _label)))
    (else
      (bind _asacf_my_current (Utilities|Casting|CastToACF_My_Current OtherActor))
      (Variables|Default|GetAs%20ACF%20My%20Current
        (:then
          _)
        (:else
          (Variables|Default|SetAs%20ACF%20My%20Current _asacf_my_current)))
      (if (not (Class|AnimInstance|IsAnyMontagePlaying (Class|ACFCharacter|GetACFAnimInstance (Variables|Default|GetAs%20ACF%20My%20Current))))
        (if (Variables|Default|GetStart/End%20Ledge?)
          ;;[0.8178 1 0] This is for starting ledges only\
          (if (not (Variables|/Game/ACF_Assets/ACF_My_Current.ACF_My_Current_C|GetOnWalkingLedge (Variables|Default|GetAs%20ACF%20My%20Current)))
            (Input|DisableInput (Variables|Default|GetAs%20ACF%20My%20Current) (Game|GetPlayerController 0))
            (Components|Movement|StopMovementImmediately (Variables|/Script/Engine.Character|GetCharacterMovement (Variables|Default|GetAs%20ACF%20My%20Current)))
            (Transformation|SetActorLocation (Variables|Default|GetAs%20ACF%20My%20Current) (Math|Vector|MakeVector _x _y (.z (Transformation|GetActorLocation (Variables|Default|GetAs%20ACF%20My%20Current)))) false false)
            (Pawn|SetControlRotation (Game|GetPlayerController 0) (Math|Rotator|MakeRotator 0.0 0.0 (.yaw (Math|Rotator|FindLookatRotation (Transformation|GetActorLocation (Variables|Default|GetAs%20ACF%20My%20Current)) (+ (* (Math|Vector|GetForwardVector (Transformation|GetWorldRotation _collisiontrigger)) -55.0) (Transformation|GetWorldLocation _collisiontrigger) (* (Math|Vector|GetRightVector _collisiontrigger) 4e+01))))))
            (Variables|/Script/Engine.PlayerController|SetInputYawScale (Game|GetPlayerController 0) 0.0)
            (Utilities|FlowControl|Delay 1.5)
            (Animation|PlayAnimMontage (Variables|Default|GetAs%20ACF%20My%20Current) "/Game/RetargetAnimations/TraversalAnimations/Traversal_LedgeWalk/RM/Montages/LedgeRight_Start.LedgeRight_Start" 1.0 "None")
            (Class|ACFCharacter|SwitchMoveset (Variables|Default|GetAs%20ACF%20My%20Current) "(TagName=\"Movesets.LedgeWalkRight\")")
            (Variables|Default|SetOnLedge true)
            (Variables|/Game/ACF_Assets/ACF_My_Current.ACF_My_Current_C|SetWalkLedge_Ref (Variables|Default|GetAs%20ACF%20My%20Current) self)))))))

(event Custom|MainCharacterEvent
  (params (Montage :type Anim%20Montage%20Object%20Reference) (bInterrupted :type Boolean))
  (bind _as_acf_my_current (Variables|Default|GetAs%20ACF%20My%20Current))
  ;[1 1 1] Montage end event player
  (if (Variables|Default|GetOnLedge)
    (Development|PrintString (Utilities|String|Append (Utilities|GetDisplayName Montage) (Utilities|GetDisplayName self)) false true "(R=1.000000,G=0.840997,B=0.924758,A=1.000000)" 88.0)
    (if (not (Variables|/Game/ACF_Assets/ACF_My_Current.ACF_My_Current_C|GetOnWalkingLedge _as_acf_my_current))
      (Input|EnableInput _as_acf_my_current (Game|GetPlayerController 0))
      (Variables|/Game/ACF_Assets/ACF_My_Current.ACF_My_Current_C|SetOnWalkingLedge _as_acf_my_current true))))

(event EventBeginPlay
  (bind _ledgedirection (Variables|Default|GetLedgeDirection))
  (bind _ledgereference_front_ (Variables|LedgeSets|GetLedgeReference%28Front%29))
  (bind _asacf_my_current (Utilities|Casting|CastToACF_My_Current (Game|GetPlayerCharacter 0)))
  (Variables|Default|SetAs%20ACF%20My%20Current _asacf_my_current)
  (EventDispatchers|AssignOnMontageEnded (Class|ACFCharacter|GetACFAnimInstance (Variables|Default|GetAs%20ACF%20My%20Current)) (delegate Custom|MainCharacterEvent))
  (Development|PrintString "OMG OMG" false true "(R=1.000000,G=0.589002,B=0.000000,A=1.000000)" 15.0)
  (Variables|Default|SetArrowTipPoint (+ (Transformation|GetWorldLocation _ledgedirection) (* (Math|Rotator|GetRotationXVector (Transformation|GetWorldRotation _ledgedirection)) (* (Variables|/Script/Engine.ArrowComponent|GetArrowLength _ledgedirection) (.x (Transformation|GetWorldScale _ledgedirection))))))
  (Utilities|FlowControl|Delay 0.2)
  (bind _keys (Utilities|Map|Keys _ledgereference_front_))
  (if (Utilities|Array|IsValidIndex _keys)
    (bind _output_get (Variables|LedgeSets|SetLedgeSelector (Utilities|Array|Get(acopy) _keys)))
    (if (.ReturnValue (Utilities|Map|Find _ledgereference_front_ _output_get))
      (Utilities|IsValid (.Value (Utilities|Map|Find _ledgereference_front_ _output_get))
        (:Is%20Valid
          _)
        (:Is%20Not%20Valid
          (Development|PrintString "There is no reference set up for the ledge. 
WalkLedge_BP::BeginPlay" false true "(R=0.942053,G=1.000000,B=0.454242,A=1.000000)" 14.0)))
      (bind _keys_2 (Utilities|Map|Keys (Variables|LedgeSets|GetLedgeReference%28Back%29) :!label _label))
      (if (Utilities|Array|IsValidIndex _keys_2)
        (bind _output_get_2 (Variables|LedgeSets|SetReverseDirection (Utilities|Array|Get(acopy) _keys_2)))
        (if (.ReturnValue (Utilities|Map|Find (Variables|LedgeSets|GetLedgeReference%28Back%29) _output_get_2))
          (Utilities|IsValid (.Value (Utilities|Map|Find (Variables|LedgeSets|GetLedgeReference%28Back%29) _output_get_2))
            (:Is%20Not%20Valid
              (Development|PrintString "Error, no reference set for ledgereference(back)" false true "(R=0.598958,G=0.000716,B=0.000716,A=1.000000)" 8.0)))
          (else
            (Development|PrintString "Error, neither front nor back reference is set up" false true "(R=0.526042,G=0.082372,B=0.099796,A=1.000000)" 14.0)))))
    (else
      (goto _label))))

(event Collision|EventActorBeginOverlap
  (params (OtherActor :type Actor%20Object%20Reference)))

(event EventTick
  (params (DeltaSeconds :type Float%20%28single-precision%29)))

(fn ConstructionScript
  (bind _ledge (Variables|Default|GetLedge))
  (bind _ledgewalk_l (Variables|Default|GetLedgeWalk_L))
  (bind _collisiontrigger (Variables|Default|GetCollisionTrigger))
  (bind _end_turn (Variables|Default|GetEnd/Turn))
  (bind _wallfront (Variables|Default|GetWallFront))
  (bind _relativelocation (Variables|/Script/Engine.SceneComponent|GetRelativeLocation _ledgewalk_l))
  (bind _relativelocation_2 (Variables|/Script/Engine.SceneComponent|GetRelativeLocation _collisiontrigger))
  (bind _relativescale3d (Variables|/Script/Engine.SceneComponent|GetRelativeScale3D _ledge))
  (bind _relativelocation_3 (Variables|/Script/Engine.SceneComponent|GetRelativeLocation _end_turn))
  (bind _relativescale3d_2 (Variables|/Script/Engine.SceneComponent|GetRelativeScale3D _wallfront))
  (if (Variables|Default|GetUseVectorSlider?)
    (Transformation|SetRelativeScale3D _ledge (Math|Vector|MakeVector (Math|Float|MapRangeClamped (.X (Math|Vector|BreakVector (Variables|Default|GetDistanceVector))) -113.0 99891.273438 0.0 1e+03) (.y _relativescale3d) (.z _relativescale3d)))
    ;[1 1 1] Simply set the relative location of the end turn to the x of the distancevector
    (Transformation|SetRelativeLocation _end_turn (Math|Vector|MakeVector (.x (Variables|Default|GetDistanceVector)) (.y _relativelocation_3) (.z _relativelocation_3)) false false)
    (Transformation|SetRelativeScale3D _wallfront (Math|Vector|MakeVector (Math|Float|MapRangeClamped (.X (Math|Vector|BreakVector (Variables|Default|GetDistanceVector))) 0.0 99891.273438 1.8 1001.5) (.y _relativescale3d_2) (.z _relativescale3d_2)))
    (Transformation|SetRelativeLocation _collisiontrigger (Math|Vector|MakeVector (* (.x (Variables|Default|GetDistanceVector)) 0.97) (.y _relativelocation_2) (.z _relativelocation_2)) false false)
    ;[1 1 1] Ledge walk animation setup
    (Transformation|SetRelativeLocation _ledgewalk_l (Math|Vector|MakeVector (* (.x (Variables|Default|GetDistanceVector)) 0.7) (.y _relativelocation) (.z _relativelocation)) false false)))

(fn PositionChecker
  (bind _returnvalue (Transformation|GetActorRotation))
  (bind _returnvalue_2 (Transformation|GetActorRotation))
  (bind _ledgereference_front_ (Variables|LedgeSets|GetLedgeReference%28Front%29))
  (bind _ledgeselector (Variables|LedgeSets|GetLedgeSelector))
  (bind (_value _returnvalue_3) (Utilities|Map|Find _ledgereference_front_ _ledgeselector))
  ;[1 1 1] Right turn section
  (if _returnvalue_3
    (Utilities|IsValid _value
      (:Is%20Valid
        (LocalVariables|SetTargetLedge_Ref _value)
        (switch Utilities|FlowControl|Switch|SwitchonWalkLedge_Directions_Enum (Variables|LedgeSets|GetLedgeSelector)
          (:NewEnumerator0
            (LocalVariables|SetTargetRotatorZ -9e+01)
            (if (Math|Float|NearlyEqual(Float) (.Yaw (Math|Rotator|BreakRotator (Math|Rotator|CombineRotators _returnvalue_2 (Math|Rotator|MakeRotator 0.0 0.0 (LocalVariables|GetTargetRotatorZ))))) (.yaw (Transformation|GetActorRotation (LocalVariables|GetTargetLedge_Ref))) 5.0)
              (if (> (Math|Vector|Distance2D(Vector) (Transformation|GetWorldLocation (Variables|Default|GetEnd/Turn)) (Transformation|GetWorldLocation (Variables|WalkLedge_BP_C|GetEntrance (LocalVariables|GetTargetLedge_Ref)))) 36.0)
                (Development|PrintString (Utilities|String|Append "(WalkLedge_Bp::Position Checker___ EventBeginPlay)  
Error, target's distance isn't close enough to the main ledge. " (Utilities|String|EnumtoString (Variables|LedgeSets|GetLedgeSelector))) false true "(R=0.911458,G=0.000000,B=0.044595,A=1.000000)" 13.0)
                (Development|PrintString (Utilities|String|ToString(Float) (Math|Vector|Distance2D(Vector) (Transformation|GetWorldLocation (Variables|Default|GetEnd/Turn)) (Transformation|GetWorldLocation (Variables|WalkLedge_BP_C|GetEntrance (LocalVariables|GetTargetLedge_Ref))))) false true "(R=0.000000,G=0.660000,B=1.000000,A=1.000000)" 4.0)
                (else
                  (Development|PrintString "Left inner is succesfully set up" false true "(R=0.000000,G=0.085369,B=1.000000,A=1.000000)" 13.0)))
              (else
                (Development|PrintString (Utilities|String|Append "(WalkLedge_Bp::Position Checker___ EventBeginPlay)  
Target setup rotation does not match this rotation." " 
Self rotation: " (Utilities|String|ToString(Float) (.Yaw (Math|Rotator|BreakRotator _returnvalue_2))) " 
" (Utilities|String|EnumtoString (Variables|LedgeSets|GetLedgeSelector)) " rotation (target): " (Utilities|String|ToString(Float) (.yaw (Transformation|GetActorRotation (LocalVariables|GetTargetLedge_Ref)))) " 
Target's rotation should be ~: " (Utilities|String|ToString(Float) (.Yaw (Math|Rotator|BreakRotator (Math|Rotator|CombineRotators _returnvalue_2 (Math|Rotator|MakeRotator 0.0 0.0 (LocalVariables|GetTargetRotatorZ))))))) false true "(R=1.000000,G=0.000000,B=0.235960,A=1.000000)" 13.0))))
          (:NewEnumerator1
            (LocalVariables|SetTargetRotatorZ -9e+01)
            (if (Math|Float|NearlyEqual(Float) (.Yaw (Math|Rotator|BreakRotator (Math|Rotator|CombineRotators _returnvalue (Math|Rotator|MakeRotator 0.0 0.0 (LocalVariables|GetTargetRotatorZ))))) (.yaw (Transformation|GetActorRotation (LocalVariables|GetTargetLedge_Ref))) 5.0)
              (if (> (Math|Vector|Distance2D(Vector) (Transformation|GetWorldLocation (Variables|Default|GetEnd/Turn)) (Transformation|GetWorldLocation (Variables|WalkLedge_BP_C|GetEntrance (LocalVariables|GetTargetLedge_Ref)))) 36.0)
                (Development|PrintString "(WalkLedge_Bp::Position Checker___ EventBeginPlay)  
Error, target's distance isn't close enough to the main ledge. LEFT OUTER" false true "(R=0.911458,G=0.000000,B=0.044595,A=1.000000)" 13.0)
                (Development|PrintString (Utilities|String|ToString(Float) (Math|Vector|Distance2D(Vector) (Transformation|GetWorldLocation (Variables|Default|GetEnd/Turn)) (Transformation|GetWorldLocation (Variables|WalkLedge_BP_C|GetEntrance (LocalVariables|GetTargetLedge_Ref))))) false true "(R=0.000000,G=0.660000,B=1.000000,A=1.000000)" 4.0)
                (else
                  (Development|PrintString "Riku" false true "(R=0.000000,G=0.085369,B=1.000000,A=1.000000)" 13.0)))
              (else
                (Development|PrintString (Utilities|String|Append "(WalkLedge_Bp::Position Checker___ EventBeginPlay)  
Target setup rotation does not match this rotation." " 
Self rotation: " (Utilities|String|ToString(Float) (.Yaw (Math|Rotator|BreakRotator _returnvalue))) " 
" (Utilities|String|EnumtoString (Variables|LedgeSets|GetLedgeSelector)) " rotation (target): " (Utilities|String|ToString(Float) (.yaw (Transformation|GetActorRotation (LocalVariables|GetTargetLedge_Ref)))) " 
Target's rotation should be ~: " (Utilities|String|ToString(Float) (.Yaw (Math|Rotator|BreakRotator (Math|Rotator|CombineRotators _returnvalue (Math|Rotator|MakeRotator 0.0 0.0 (LocalVariables|GetTargetRotatorZ))))))) false true "(R=1.000000,G=0.000000,B=0.235960,A=1.000000)" 13.0))))
          (:NewEnumerator2
            (bind _output_get (LocalVariables|SetTargetRotatorZ 9e+01))
            (if (Math|Rotator|Equal(Rotator) (Math|Rotator|CombineRotators (Transformation|GetActorRotation) (Math|Rotator|MakeRotator 0.0 0.0 _output_get)) (Transformation|GetActorRotation (LocalVariables|GetTargetLedge_Ref)) 5.0)
              (if (< (Math|Vector|Distance2D(Vector) (Transformation|GetWorldLocation (Variables|Default|GetEnd/Turn)) (Transformation|GetWorldLocation (Variables|WalkLedge_BP_C|GetEntrance (LocalVariables|GetTargetLedge_Ref)))) 35.0)
                (Development|PrintString "Right inner successful" false true "(R=1.000000,G=0.340827,B=0.230999,A=1.000000)" 6.0)
                (else
                  (Development|PrintString (Utilities|String|Append "Target ledge(Right inner) isnt close enough to the main ledge" (Utilities|String|ToString(Float) (Math|Vector|Distance2D(Vector) (Transformation|GetWorldLocation (Variables|Default|GetEnd/Turn)) (Transformation|GetWorldLocation (Variables|WalkLedge_BP_C|GetEntrance (LocalVariables|GetTargetLedge_Ref)))))) false true "(R=1.000000,G=0.017682,B=0.000000,A=1.000000)" 12.0)))
              (else
                (Development|PrintString "Right inner rotation doesn't match" false true "(R=1.000000,G=0.000000,B=0.123857,A=1.000000)" 12.0))))
          (:NewEnumerator3
            (LocalVariables|SetTargetRotatorZ 9e+01)
            (if (Math|Rotator|Equal(Rotator) (Math|Rotator|CombineRotators (Transformation|GetActorRotation) (Math|Rotator|MakeRotator 0.0 0.0 (LocalVariables|GetTargetRotatorZ))) (Transformation|GetActorRotation (LocalVariables|GetTargetLedge_Ref)) 5.0)
              (if (not (< (Math|Vector|Distance2D(Vector) (Transformation|GetWorldLocation (Variables|Default|GetEntrance)) (Transformation|GetWorldLocation (Variables|WalkLedge_BP_C|GetEnd/Turn (LocalVariables|GetTargetLedge_Ref)))) 37.0))
                (Development|PrintString (Utilities|String|Append "Error, targets ledge is not close enough to the main ledge. 
WalkLedge_BP::Position Checker Event Begin Play Right Outer" "") false true "(R=0.258183,G=0.000304,B=0.000304,A=1.000000)"))
              (else
                (Development|PrintString (Utilities|String|Append (Utilities|String|EnumtoString (Variables|LedgeSets|GetLedgeSelector)) " rotation error.") false true "(R=0.300544,G=0.000000,B=0.000000,A=1.000000)" 7.0)))))))))

(fn BreakLinktoLedge
  (params (SwitchLedge? :type Boolean) (Front%20Ledge? :type Boolean))
  (bind _ledgereference_front_ (Variables|LedgeSets|GetLedgeReference%28Front%29))
  (bind _ledgeselector (Variables|LedgeSets|GetLedgeSelector))
  (bind _ledgereference_back_ (Variables|LedgeSets|GetLedgeReference%28Back%29))
  (bind _reversedirection (Variables|LedgeSets|GetReverseDirection))
  (bind _value (Utilities|Map|Find _ledgereference_front_ _ledgeselector))
  (bind _value_2 (Utilities|Map|Find _ledgereference_back_ _reversedirection))
  (bind _as_acf_my_current (Variables|Default|GetAs%20ACF%20My%20Current)
    (:then
      (if SwitchLedge?
        (if Front%20Ledge?
          (bind _output_get (Variables|/Game/ACF_Assets/ACF_My_Current.ACF_My_Current_C|SetWalkLedge_Ref _as_acf_my_current _value))
          (Variables|Default|SetOnLedge false)
          (Pawn|SetControlRotation (Game|GetPlayerController 0) (Math|Rotator|MakeRotator 0.0 0.0 (.yaw (Transformation|GetActorRotation _output_get))))
          (Variables|WalkLedge_BP_C|SetOnLedge _value true)
          (else
            (bind _output_get_2 (Variables|/Game/ACF_Assets/ACF_My_Current.ACF_My_Current_C|SetWalkLedge_Ref _as_acf_my_current _value_2))
            (Variables|Default|SetOnLedge false)
            (Pawn|SetControlRotation (Game|GetPlayerController 0) (Math|Rotator|MakeRotator 0.0 0.0 (.yaw (Math|Rotator|CombineRotators (Transformation|GetActorRotation _output_get_2) "0,180.000000, 0"))))
            (Variables|WalkLedge_BP_C|SetOnLedge _value_2 true)))
        (else
          (Class|ACFCharacter|SwitchMoveset _as_acf_my_current "(TagName=\"Movesets\")")
          (Variables|/Game/ACF_Assets/ACF_My_Current.ACF_My_Current_C|SetWalkLedge_Ref _as_acf_my_current 0)
          (bind _output_get_3 (Variables|/Game/ACF_Assets/ACF_My_Current.ACF_My_Current_C|SetOnWalkingLedge _as_acf_my_current false))
          (Variables|Default|SetOnLedge _output_get_3)
          (Variables|/Script/Engine.PlayerController|SetInputYawScale (Game|GetPlayerController 0) 1.0))))
    (:else
      (Development|PrintString (Utilities|String|Append "For some reason, player reference isn't valid. (WalkLedge_BP::Break Link to Ledge)" " 
Object name: " (Utilities|GetObjectName self)) false true "(R=1.000000,G=0.042603,B=0.000000,A=1.000000)" 12.0))))